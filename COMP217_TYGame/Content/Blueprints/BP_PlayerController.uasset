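; Player controller for a third-person shooter that handles the death, game over and win end states.
; Each state unpossesses the pawn, fades the camera to full and shows the WBP_GameOver widget, followed by a short delay.
; OnDeath and GameOver share one path that then removes the widget and calls RestartGame on ThirdPersonShooterMode.
; WinState reuses the game-over widget but ends after the delay without removing it or restarting.
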(event Custom|OnDeath
  (Pawn|UnPossess)
  (CameraFades|StartCameraFade :self (Variables|Default|GetPlayerCameraManager) :ToAlpha 1.0 :Duration 1.0 :bHoldWhenFinished true)
  (bind _returnvalue (UserInterface|CreateWidget "/Game/WBP_GameOver.WBP_GameOver_C" self))
  (UserInterface|Viewport|AddtoViewport _returnvalue 0)
  (Utilities|FlowControl|Delay 3.0)
  (Widget|RemovefromParent _returnvalue)
  (bind _asthird_person_shooter_mode (Utilities|Casting|CastToThirdPersonShooterMode (Game|GetGameMode)))
  (Class|GameMode|RestartGame _asthird_person_shooter_mode))

(event Custom|GameOver
  (Pawn|UnPossess)
  (CameraFades|StartCameraFade :self (Variables|Default|GetPlayerCameraManager) :ToAlpha 1.0 :Duration 1.0 :bHoldWhenFinished true)
  (bind _returnvalue (UserInterface|CreateWidget "/Game/WBP_GameOver.WBP_GameOver_C" self))
  (UserInterface|Viewport|AddtoViewport _returnvalue 0)
  (Utilities|FlowControl|Delay 3.0)
  (Widget|RemovefromParent _returnvalue)
  (bind _asthird_person_shooter_mode (Utilities|Casting|CastToThirdPersonShooterMode (Game|GetGameMode)))
  (Class|GameMode|RestartGame _asthird_person_shooter_mode))

(event Custom|WinState
  (Pawn|UnPossess)
  (CameraFades|StartCameraFade :self (Variables|Default|GetPlayerCameraManager) :ToAlpha 1.0 :Duration 1.0 :bHoldWhenFinished true)
  (bind _returnvalue (UserInterface|CreateWidget "/Game/WBP_GameOver.WBP_GameOver_C" self))
  (UserInterface|Viewport|AddtoViewport _returnvalue 0)
  (Utilities|FlowControl|Delay 3.0))

(event EventBeginPlay)

(event EventTick
  (params (DeltaSeconds :type Float%20%28single-precision%29)))

(fn ConstructionScript)