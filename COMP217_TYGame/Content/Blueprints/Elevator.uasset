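; Elevator actor that rises while something overlaps its Box trigger and descends otherwise.
; Unfiltered begin and end overlap events toggle IsPlayerOn, which Tick checks against hardcoded world-Z limits to set Speed's sign before calling MoveUp, whose body is not shown.
; At the upper limit the descend branch also runs while occupied, so the platform oscillates there instead of stopping.
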(event OnComponentBeginOverlap(Box)
  (params (OverlappedComponent :type Primitive%20Component%20Object%20Reference) (OtherActor :type Actor%20Object%20Reference) (OtherComp :type Primitive%20Component%20Object%20Reference) (OtherBodyIndex :type Integer) (bFromSweep :type Boolean) (SweepResult :type Hit%20Result%20Structure%20%28by%20ref%29))
  (Variables|Default|SetisPlayerOn true))

(event OnComponentEndOverlap(Box)
  (params (OverlappedComponent :type Primitive%20Component%20Object%20Reference) (OtherActor :type Actor%20Object%20Reference) (OtherComp :type Primitive%20Component%20Object%20Reference) (OtherBodyIndex :type Integer))
  (Variables|Default|SetisPlayerOn false))

(event EventBeginPlay)

(event Collision|EventActorBeginOverlap
  (params (OtherActor :type Actor%20Object%20Reference)))

(event EventTick
  (params (DeltaSeconds :type Float%20%28single-precision%29))
  (bind _returnvalue (Transformation|GetActorLocation))
  (bind _z (Math|Vector|BreakVector _returnvalue))
  (if (and (Variables|Default|GetisPlayerOn) (< _z 315.0))
    (Variables|Default|Setspeed 1.0)
    (Class|ElevatorPlatform|MoveUp :!label _label)
    (elif (> _z 3e+01)
      (Variables|Default|Setspeed -1.0)
      (goto _label))))

(fn ConstructionScript)