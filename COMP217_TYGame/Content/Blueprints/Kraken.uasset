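; Kraken actor that works as a one-shot explosive hazard, hurting whatever overlaps its trigger.
; On overlap it spawns an explosion effect at the trigger's transform and sends a fixed damage message to the other actor.
; It then destroys its mesh and trigger components, leaving the actor itself alive, as the DestroyActor and end-play binding nodes are never run.
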(event OnComponentHit(Trigger)
  (params (HitComponent :type Primitive%20Component%20Object%20Reference) (OtherActor :type Actor%20Object%20Reference) (OtherComp :type Primitive%20Component%20Object%20Reference) (NormalImpulse :type Vector :default "0, 0, 0") (Hit :type Hit%20Result%20Structure%20%28by%20ref%29)))

(event OnComponentBeginOverlap(Trigger)
  (params (OverlappedComponent :type Primitive%20Component%20Object%20Reference) (OtherActor :type Actor%20Object%20Reference) (OtherComp :type Primitive%20Component%20Object%20Reference) (OtherBodyIndex :type Integer) (bFromSweep :type Boolean) (SweepResult :type Hit%20Result%20Structure%20%28by%20ref%29))
  (Utilities|FlowControl|Sequence
    (:then_0
      (Game|SpawnActorfromClass "/Game/StarterContent/Blueprints/Blueprint_Effect_Explosion.Blueprint_Effect_Explosion_C" (Transformation|GetWorldTransform (Variables|Default|GetTrigger)) "Undefined" 0 0)
      (Variables|Default|SetExplosion%20Effect 0)
      (Class|BPIDamagabale|TakeDamage(Message) OtherActor 2e+01))
    (:then_1
      (Components|DestroyComponent (Variables|Default|GetKrakenMesh)))))

(event Custom|OnEndPlay_Event_0
  (params (Actor :type Actor%20Object%20Reference) (EndPlayReason :type EEndPlayReason%20Enum :default "Destroyed")))

(event EventBeginPlay)

(event Collision|EventActorBeginOverlap
  (params (OtherActor :type Actor%20Object%20Reference)))

(event EventTick
  (params (DeltaSeconds :type Float%20%28single-precision%29)))

(fn ConstructionScript)